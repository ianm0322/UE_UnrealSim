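; Player pawn for the playground: a spring-arm camera rig with planar movement, rotation and zoom.
; BeginPlay adds the Enhanced Input mapping context and seeds the targets from the current location, rotation and arm length.
; Input only changes those targets: movement follows the pawn's rotation, zoom is clamped, and look left/right rotates in 45-degree steps.
; Tick interpolates the pawn and arm length toward the targets, with separate smoothness for each.
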(event `self.ReceiveBeginPlay`
  (`self.InitializeInput`)
  (set `self.mTargetMovement` (`self.K2_GetActorLocation`))
  (set `self.mTargetZoomValue` (`SpringArmComponent.TargetArmLength` (`self.SpringArm`)))
  (set `self.mTargetRotation` (`self.K2_GetActorRotation`)))

(event `self.ReceiveTick`
  (params (DeltaSeconds :type "Float (single-precision)"))
  (bind _springarm (`self.SpringArm`))
  (set `SpringArmComponent.TargetArmLength` (`KismetMathLibrary.FInterpTo` (`SpringArmComponent.TargetArmLength` _springarm) (`self.mTargetZoomValue`) DeltaSeconds (`self.ZoomSmoothness`)) _springarm)
  (`self.K2_SetActorLocation` (`KismetMathLibrary.VInterpTo` (`self.K2_GetActorLocation`) (`self.mTargetMovement`) DeltaSeconds (`self.MoveSmoothness`)))
  (`self.K2_SetActorRotation` (`KismetMathLibrary.RInterpTo` (`self.K2_GetActorRotation`) (`self.mTargetRotation`) DeltaSeconds (`self.RotationSmoothness`))))

(event `EnhancedInput|/Game/01_UnrealSim/01_PlayGround/04_Input/Camera/IA_PG_Zoom`
  (params (ActionValue :type "Float (double-precision)") (ElapsedSeconds :type "Float (double-precision)") (TriggeredSeconds :type "Float (double-precision)") (InputAction :type "InputAction Object Reference" :default "/Game/01_UnrealSim/01_PlayGround/04_Input/Camera/IA_PG_Zoom.IA_PG_Zoom"))
  ;[1 1 1] Camera Zooming
  (:`Triggered`
    (`self.ZoomCamera` ActionValue :!label _label) ; (curr) + (ZoomSpeed) * (Input) | (MinZoom)..(MaxZoom)
  )
  (:`Canceled`
    (goto _label))
  (:`Completed`
    (goto _label)))

(event `EnhancedInput|/Game/01_UnrealSim/01_PlayGround/04_Input/Control/IA_PG_MoveOnPlane`
  (params (ActionValue :type "Vector2D Structure") (ElapsedSeconds :type "Float (double-precision)") (TriggeredSeconds :type "Float (double-precision)") (InputAction :type "InputAction Object Reference" :default "/Game/01_UnrealSim/01_PlayGround/04_Input/Control/IA_PG_MoveOnPlane.IA_PG_MoveOnPlane"))
  (bind (_returnvalue_x _returnvalue_y) (`KismetMathLibrary.BreakVector2D` (* ActionValue (`self.MoveSpeed`))))
  ;[1 1 1] Set Target Location
  (:`Triggered`
    (set `self.mTargetMovement` (+ (`self.mTargetMovement`) (* (`KismetMathLibrary.GreaterGreater_VectorRotator` (`KismetMathLibrary.MakeVector` _returnvalue_y _returnvalue_x) (`self.K2_GetActorRotation`)) (`self.MoveSpeed`) (`GameplayStatics.GetWorldDeltaSeconds`))))))

(event `EnhancedInput|/Game/01_UnrealSim/01_PlayGround/04_Input/Control/IA_PG_Rotation`
  (params (ActionValue :type "Vector2D Structure") (ElapsedSeconds :type "Float (double-precision)") (TriggeredSeconds :type "Float (double-precision)") (InputAction :type "InputAction Object Reference" :default "/Game/01_UnrealSim/01_PlayGround/04_Input/Control/IA_PG_Rotation.IA_PG_Rotation"))
  (bind (_x _y) (`KismetMathLibrary.BreakVector2D` ActionValue))
  ;[1 1 1] Set Rotation
  (:`Triggered`
    (set `self.mTargetRotation` (`KismetMathLibrary.ComposeRotators` (`self.mTargetRotation`) (`KismetMathLibrary.MakeRotator` 0.0 _y _x)))))

(event `EnhancedInput|/Game/01_UnrealSim/01_PlayGround/04_Input/Control/IA_PG_Rotation_LookLeft`
  (params (ActionValue :type Boolean) (ElapsedSeconds :type "Float (double-precision)") (TriggeredSeconds :type "Float (double-precision)") (InputAction :type "InputAction Object Reference" :default "/Game/01_UnrealSim/01_PlayGround/04_Input/Control/IA_PG_Rotation_LookLeft.IA_PG_Rotation_LookLeft"))
  ;[1 1 1] Set Rotation
  (:`Triggered`
    (set `self.mTargetRotation` (`KismetMathLibrary.ComposeRotators` (`self.mTargetRotation`) (struct :`Yaw` -45.0)))))

(event `EnhancedInput|/Game/01_UnrealSim/01_PlayGround/04_Input/Control/IA_PG_Rotation_LookRight`
  (params (ActionValue :type Boolean) (ElapsedSeconds :type "Float (double-precision)") (TriggeredSeconds :type "Float (double-precision)") (InputAction :type "InputAction Object Reference" :default "/Game/01_UnrealSim/01_PlayGround/04_Input/Control/IA_PG_Rotation_LookRight.IA_PG_Rotation_LookRight"))
  ;[1 1 1] Set Rotation
  (:`Triggered`
    (set `self.mTargetRotation` (`KismetMathLibrary.ComposeRotators` (`self.mTargetRotation`) (struct :`Yaw` 45.0)))))

(fn `InitializeInput`
  (bind _asplayer_controller (cast `PlayerController` (`self.GetController`)))
  (`EnhancedInputSubsystemInterface.AddMappingContext` (pcsubsystem `EnhancedInputLocalPlayerSubsystem` _asplayer_controller) "/Game/01_UnrealSim/01_PlayGround/04_Input/IMC_PG_Default.IMC_PG_Default" 0 (struct)))

(fn `UserConstructionScript`)

(fn `ZoomCamera`
  (params (Input :type "Float (double-precision)"))
  (set `self.mTargetZoomValue` (`KismetMathLibrary.FClamp` (+ (* Input (`self.ZoomSpeed`)) (`self.mTargetZoomValue`)) (`self.MinZoom`) (`self.MaxZoom`))))